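; HUD Blueprint that shows ammo for the player's current weapon.
; It creates a weapon UI widget and adds it to the viewport on BeginPlay.
; Every Tick it casts the owning pawn to BP_ProtagClass and copies the CurrentAmmo and AmmoCount of the equipped WeaponInventory entry into the widget, polling rather than responding to events.
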(event EventBeginPlay
  (bind _returnvalue (UserInterface|CreateWidget "/Game/UI/WeaponUI.WeaponUI_C"))
  (UserInterface|Viewport|AddtoViewport _returnvalue 0))

(event Collision|EventActorBeginOverlap
  (params (OtherActor :type Actor%20Object%20Reference)))

(event EventTick
  (params (DeltaSeconds :type Float%20%28single-precision%29))
  (bind _asbp_protag_class (Utilities|Casting|CastToBP_ProtagClass (Class|HUD|GetOwningPawn)))
  (Utilities|FlowControl|Sequence
    (:then_0
      (Variables|/Game/UI/WeaponUI.WeaponUI_C|SetAmmoCurrent (stale EventBeginPlay _returnvalue) (Variables|/Script/MovementDemo.WeaponBase|GetCurrentAmmo (Utilities|Array|Get(acopy) (Variables|/Script/MovementDemo.ProtagClass|GetWeaponInventory _asbp_protag_class) (Variables|/Script/MovementDemo.ProtagClass|Getcurrent_weapon _asbp_protag_class)))))
    (:then_1
      (Variables|/Game/UI/WeaponUI.WeaponUI_C|SetAmmoTotal (stale EventBeginPlay _returnvalue) (Variables|/Script/MovementDemo.WeaponBase|GetAmmoCount (Utilities|Array|Get(acopy) (Variables|/Script/MovementDemo.ProtagClass|GetWeaponInventory _asbp_protag_class) (Variables|/Script/MovementDemo.ProtagClass|Getcurrent_weapon _asbp_protag_class)))))))

(fn ConstructionScript)