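; Game mode for the movement demo that also drives a makeshift ammo HUD, marked in the graph as needing a fix.
; BeginPlay creates a WeaponUI widget and adds it to the viewport.
; Every Tick it casts player 0's pawn to BP_ProtagClass and copies the current weapon's loaded and total ammo from WeaponInventory into the widget, polling rather than using events.
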(event EventBeginPlay
  ;[1 1 1] shitty ammo ui, fix me
  (bind _returnvalue (UserInterface|CreateWidget "/Game/UI/WeaponUI.WeaponUI_C"))
  (UserInterface|Viewport|AddtoViewport _returnvalue 0))

(event EventTick
  (params (DeltaSeconds :type Float%20%28single-precision%29))
  ;[1 1 1] shitty ammo ui, fix me
  (bind _asbp_protag_class (Utilities|Casting|CastToBP_ProtagClass (Game|Player|GetPlayerPawn 0)))
  (Variables|/Game/UI/WeaponUI.WeaponUI_C|SetAmmoCurrent (stale EventBeginPlay _returnvalue) (Variables|/Script/MovementDemo.WeaponBase|GetCurrentAmmo (Utilities|Array|Get(acopy) (Variables|/Script/MovementDemo.ProtagClass|GetWeaponInventory _asbp_protag_class) (Variables|/Script/MovementDemo.ProtagClass|Getcurrent_weapon _asbp_protag_class))))
  (Variables|/Game/UI/WeaponUI.WeaponUI_C|SetAmmoTotal (stale EventBeginPlay _returnvalue) (Variables|/Script/MovementDemo.WeaponBase|GetAmmoCount (Utilities|Array|Get(acopy) (Variables|/Script/MovementDemo.ProtagClass|GetWeaponInventory _asbp_protag_class) (Variables|/Script/MovementDemo.ProtagClass|Getcurrent_weapon _asbp_protag_class)))))

(fn ConstructionScript)